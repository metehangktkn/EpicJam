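; In-game game mode for a floor-based game, where each floor is a separate level named "L_" plus its index.
; On begin play it shows the W_Floors widget and tells BP_GameInstance the level is ready.
; The construction script maps each BP_PlayerStart by its Direction.
; ChoosePlayerStart picks one by floor change: one down, one up, or a shared start for same-floor and multi-floor jumps.
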(event `self.ReceiveBeginPlay`
  (bind _returnvalue (`|CreateWidget` "/Game/Blueprints/Floor/Widget/W_Floors.W_Floors_C"))
  (`UserWidget.AddToViewport` _returnvalue 0)
  (bind _asbp_game_instance (cast `/Game/Blueprints/GameMode/BP_GameInstance` (`GameplayStatics.GetGameInstance`)))
  (`/Game/Blueprints/GameMode/BP_GameInstance.Level Ready` _asbp_game_instance))

(fn `ChoosePlayerStart`
  (params (Player :type "Controller Object Reference"))
  (returns (ReturnValue :type "Actor Object Reference"))
  (return (`self.GetPlayerStart`)))

(fn `GetPlayerStart`
  (returns (PlayerStart :type "Actor Object Reference"))
  (bind _playerstarts (`self.PlayerStarts`))
  (bind _returnvalue (- (`/Game/Blueprints/GeneralFunctions.GetCurrentFloorIndex`) (`/Game/Blueprints/GeneralFunctions.GetPreviousFloorIndex`)))
  (return (select `bool` (== (- (`/Game/Blueprints/GeneralFunctions.GetCurrentFloorIndex`) (`/Game/Blueprints/GeneralFunctions.GetPreviousFloorIndex`)) 0) :`false` (select `bool` (> (`KismetMathLibrary.Abs_Int` _returnvalue) 1) :`false` (select `bool` (== _returnvalue -1) :`false` (`BlueprintMapLibrary.Map_Find` _playerstarts "NewEnumerator1") :`true` (`BlueprintMapLibrary.Map_Find` _playerstarts "NewEnumerator0") :!type "Actor Object Reference") :`true` (`BlueprintMapLibrary.Map_Find` _playerstarts "NewEnumerator2") :!type "Actor Object Reference") :`true` (`BlueprintMapLibrary.Map_Find` (`self.PlayerStarts`) "NewEnumerator2") :!type "Actor Object Reference")))

(fn `SetPlayerFloorIndex`
  (params (PlayerFloorIndex :type Integer))
  (set `self.PlayerFloorIndex` PlayerFloorIndex))

(fn `TravelToFloor`
  (params (Index :type Integer))
  (`GameplayStatics.OpenLevel` (`KismetStringLibrary.Conv_StringToName` (`KismetStringLibrary.Concat_StrStr` "L_" (`KismetStringLibrary.Conv_IntToString` Index)))))

(fn `UserConstructionScript`
  (`parent.UserConstructionScript`)
  (bind _outactors (`GameplayStatics.GetAllActorsOfClass` "/Game/Blueprints/Floor/BP_PlayerStart.BP_PlayerStart_C"))
  (for _array_element _outactors
    (`BlueprintMapLibrary.Map_Add` (`self.PlayerStarts`) (`/Game/Blueprints/Floor/BP_PlayerStart.Direction` _array_element) _array_element)))