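; Actor component that manages a player's inventory and equipment, registering its UI widget on the P key at BeginPlay.
; Items live in per-type arrays, with limited equipment slots and an ID map tracking location and index, which is not reindexed after removals.
; Transfers update stat totals by category and addition type and fire change events.
; ApplyStats pushes totals to equipped item actors, though the actor-spawning branch is disconnected.
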(event `self.ReceiveBeginPlay`
  (bind _returnvalue (`|CreateWidget` "/Game/Blueprints/InventoryEquipment/Widget/W_InventoryEquipment.W_InventoryEquipment_C" null null))
  (message `/Game/Blueprints/Player/Interface/BPI_PlayerController.AddWidget` (`GameplayStatics.GetPlayerController` 0) "P" _returnvalue))

(fn `AddItemStats`
  (params (Item :type "/Game/Blueprints/InventoryEquipment/Struct/S_Item Structure"))
  (locals (AddedAmount :type "Float (double-precision)") (Stat :type "/Game/Blueprints/InventoryEquipment/Struct/S_ItemStats Structure") (AmountsRef :type "Map of /Game/Blueprints/InventoryEquipment/Enum/E_StatAdditionType Enum to Float (double-precision)"))
  (bind ((`StatCategory_8_E8BBAE9D48BEC6D0801E889EF8F0BA87` _statcategory) (`StatAdditionType_2_29FFFC8F41736F431C31B68AAD5BE0B5` _statadditiontype)) (break `/Game/Blueprints/InventoryEquipment/Struct/S_ItemStats` (`local.Stat`)))
  (for _array_element (`.Stats_46_BD9FFE044F6D0BF1D424B09076C86854` (break `/Game/Blueprints/InventoryEquipment/Struct/S_Item` Item))
    (bind _output_get (set `local.Stat` _array_element))
    (bind (_statcategory_2 _statadditiontype_2 _statamount) (break `/Game/Blueprints/InventoryEquipment/Struct/S_ItemStats` _output_get))
    (bind _amounts (break `/Game/Blueprints/InventoryEquipment/Struct/S_StatAmounts` (`BlueprintMapLibrary.Map_Find` (`self.Stats`) _statcategory_2)))
    (set `local.AmountsRef` _amounts)
    (bind _output_get_2 (set `local.AddedAmount` (+ (`BlueprintMapLibrary.Map_Find` _amounts _statadditiontype_2) _statamount)))
    (`BlueprintMapLibrary.Map_Add` (`local.AmountsRef`) _statadditiontype _output_get_2)
    (`BlueprintMapLibrary.Map_Add` (`self.Stats`) _statcategory (make `/Game/Blueprints/InventoryEquipment/Struct/S_StatAmounts` (`local.AmountsRef`))))
  (`self.StatsChanged` (`self.Stats`) true))

(fn `AddItemToEquipment`
  (params (Item :type "/Game/Blueprints/InventoryEquipment/Struct/S_Item Structure"))
  (returns (Added :type Boolean))
  (locals (ItemRef :type "/Game/Blueprints/InventoryEquipment/Struct/S_Item Structure") (ItemTypeRef :type "/Game/Blueprints/InventoryEquipment/Enum/E_ItemType Enum") (ItemArrayRef :type "Array of /Game/Blueprints/InventoryEquipment/Struct/S_Item Structure") (ItemEquipmentIndex :type Integer :default 0) (ItemLocationRef :type "/Game/Blueprints/InventoryEquipment/Struct/S_ItemLocation Structure") (ItemActorRef :type "/Game/Blueprints/InventoryEquipment/Item/BP_ItemBase Object Reference"))
  (bind _output_get (set `local.ItemRef` Item))
  (bind _output_get_2 (set `local.ItemTypeRef` (`.ItemType_35_B85020CC4326255BF9CA7986369ED08C` (break `/Game/Blueprints/InventoryEquipment/Struct/S_Item` _output_get))))
  (bind _isthere (`self.IsThereEmptySlotInEquipment` _output_get_2))
  (if _isthere
    (bind _output_get_3 (set `local.ItemArrayRef` (`.Array_3_54825DA340DDAE3ADDAE89ABB7425895` (break `/Game/Blueprints/InventoryEquipment/Struct/S_ItemArray` (`BlueprintMapLibrary.Map_Find` (`self.EquipmentArray`) (`local.ItemTypeRef`))))))
    (bind _returnvalue (`KismetArrayLibrary.Array_Add` _output_get_3 (`local.ItemRef`)))
    (set `local.ItemEquipmentIndex` _returnvalue)
    (`BlueprintMapLibrary.Map_Add` (`self.EquipmentArray`) (`local.ItemTypeRef`) (make `/Game/Blueprints/InventoryEquipment/Struct/S_ItemArray` (`local.ItemArrayRef`)))
    (`KismetArrayLibrary.Array_Clear` (`local.ItemArrayRef`))
    (bind _output_get_4 (set `local.ItemLocationRef` (`BlueprintMapLibrary.Map_Find` (`self.InventoryIDs`) (`.ID_34_480AFE364D7F3357C84857B4B302F81E` (break `/Game/Blueprints/InventoryEquipment/Struct/S_Item` (`local.ItemRef`))))))
    (bind _structout (setmembers `/Game/Blueprints/InventoryEquipment/Struct/S_ItemLocation` :`StructRef` _output_get_4 :`ItemLocation` "NewEnumerator1" :`Index` (`local.ItemEquipmentIndex`)))
    (`BlueprintMapLibrary.Map_Add` (`self.InventoryIDs`) (`.ID_34_480AFE364D7F3357C84857B4B302F81E` (break `/Game/Blueprints/InventoryEquipment/Struct/S_Item` (`local.ItemRef`))) _structout)
    (`self.AddItemStats` (`local.ItemRef`))
    (`self.ItemAddedToEquipment` (`local.ItemRef`))
    (return true)
    (else
      (return false))))

(fn `AddItemToInventory`
  (params (Item :type "/Game/Blueprints/InventoryEquipment/Struct/S_Item Structure"))
  (returns (Added :type Boolean))
  (locals (ItemRef :type "/Game/Blueprints/InventoryEquipment/Struct/S_Item Structure") (ItemTypeRef :type "/Game/Blueprints/InventoryEquipment/Enum/E_ItemType Enum") (ItemArrayRef :type "Array of /Game/Blueprints/InventoryEquipment/Struct/S_Item Structure") (ItemInventoryIndex :type Integer :default 0) (ItemLocationRef :type "/Game/Blueprints/InventoryEquipment/Struct/S_ItemLocation Structure"))
  (bind ((`ID_34_480AFE364D7F3357C84857B4B302F81E` _id) (`ItemType_35_B85020CC4326255BF9CA7986369ED08C` _itemtype)) (break `/Game/Blueprints/InventoryEquipment/Struct/S_Item` (`local.ItemRef`)))
  (bind ((`ItemInstance_49_12CEFC5A48A041FEE90347952F911701` _iteminstance)) (break `/Game/Blueprints/InventoryEquipment/Struct/S_Item` (`local.ItemRef`)))
  (bind _output_get (set `local.ItemRef` Item))
  (if (== (`.ID_34_480AFE364D7F3357C84857B4B302F81E` (break `/Game/Blueprints/InventoryEquipment/Struct/S_Item` _output_get)) -1)
    (setmembers `/Game/Blueprints/InventoryEquipment/Struct/S_Item` :`StructRef` (`local.ItemRef`) :`ID` (`self.CreateANewID`)))
  (`/Engine/EditorBlueprintResources/StandardMacros.IsValid` _iteminstance
    (:`Is Valid`
      (`Actor.K2_DestroyActor` _iteminstance))
    (:`Is Not Valid`
      _))
  (set `local.ItemTypeRef` (`.ItemType_35_B85020CC4326255BF9CA7986369ED08C` (break `/Game/Blueprints/InventoryEquipment/Struct/S_Item` (`local.ItemRef`))))
  (bind _output_get_2 (set `local.ItemArrayRef` (`.Array_3_54825DA340DDAE3ADDAE89ABB7425895` (break `/Game/Blueprints/InventoryEquipment/Struct/S_ItemArray` (`BlueprintMapLibrary.Map_Find` (`self.InventoryArray`) (`local.ItemTypeRef`))))))
  (bind _returnvalue (`KismetArrayLibrary.Array_Add` _output_get_2 (`local.ItemRef`)))
  (set `local.ItemInventoryIndex` _returnvalue)
  (`BlueprintMapLibrary.Map_Add` (`self.InventoryArray`) (`local.ItemTypeRef`) (make `/Game/Blueprints/InventoryEquipment/Struct/S_ItemArray` (`local.ItemArrayRef`)))
  (`KismetArrayLibrary.Array_Clear` (`local.ItemArrayRef`))
  (`BlueprintMapLibrary.Map_Add` (`self.InventoryIDs`) _id (make `/Game/Blueprints/InventoryEquipment/Struct/S_ItemLocation` "NewEnumerator0" _itemtype (`local.ItemInventoryIndex`)))
  (`self.ItemAddedToInventory` (`local.ItemRef`))
  (return true))

(fn `ApplyStats`
  (params (Stats :type "Map of /Game/Blueprints/InventoryEquipment/Enum/E_StatCategory Enum to /Game/Blueprints/InventoryEquipment/Struct/S_StatAmounts Structure"))
  (locals (StatCategoryRef :type "/Game/Blueprints/InventoryEquipment/Enum/E_StatCategory Enum") (ItemRef :type "/Game/Blueprints/InventoryEquipment/Struct/S_Item Structure"))
  (bind ((`ItemInstance_49_12CEFC5A48A041FEE90347952F911701` _iteminstance)) (break `/Game/Blueprints/InventoryEquipment/Struct/S_Item` (`local.ItemRef`)))
  (bind _keys (`BlueprintMapLibrary.Map_Keys` Stats))
  (for _array_element _keys
    (set `local.StatCategoryRef` _array_element)
    (bind _keys_2 (`BlueprintMapLibrary.Map_Keys` (`self.EquipmentArray`)))
    (for _array_element_2 _keys_2
      (for _array_element_3 (`.Array_3_54825DA340DDAE3ADDAE89ABB7425895` (break `/Game/Blueprints/InventoryEquipment/Struct/S_ItemArray` (`BlueprintMapLibrary.Map_Find` (`self.EquipmentArray`) _array_element_2)))
        (bind _output_get (set `local.ItemRef` _array_element_3))
        (if (!= (`KismetArrayLibrary.Array_Find` (`.AffectedStats_57_522A3D5A42A4F06C3A353285C3431348` (break `/Game/Blueprints/InventoryEquipment/Struct/S_Item` _output_get)) (`local.StatCategoryRef`)) -1)
          (`/Engine/EditorBlueprintResources/StandardMacros.IsValid` _iteminstance
            (:`Is Valid`
              (`/Game/Blueprints/InventoryEquipment/Interface/BPI_ItemInterface.ChangeStat` _iteminstance (`local.StatCategoryRef`) (`BlueprintMapLibrary.Map_Find` (`.Amounts_26_0915A13F4F6A65445893A8A768B38F02` (break `/Game/Blueprints/InventoryEquipment/Struct/S_StatAmounts` (`BlueprintMapLibrary.Map_Find` (`local.Stats`) (`local.StatCategoryRef`)))) "NewEnumerator0")))))))))

(fn `CreateANewID`
  (returns (ID :type Integer))
  (bind _keys (`BlueprintMapLibrary.Map_Keys` (`self.InventoryIDs`)))
  (return (+ (`.MaxValue` (`KismetMathLibrary.MaxOfIntArray` _keys)) 1)))

(fn `GetItem`
  (params (ID :type Integer))
  (returns (Item :type "/Game/Blueprints/InventoryEquipment/Struct/S_Item Structure (by ref)"))
  (locals (ItemLocationRef :type "/Game/Blueprints/InventoryEquipment/Struct/S_ItemLocation Structure"))
  (bind ((`ItemType_2_942F781946676B764945B0BB0CB8F2C5` _itemtype) (`Index_5_8D07E8A340549BCF8C93F5A33213EC03` _index)) (break `/Game/Blueprints/InventoryEquipment/Struct/S_ItemLocation` (`local.ItemLocationRef`)))
  (bind _output_get (set `local.ItemLocationRef` (`BlueprintMapLibrary.Map_Find` (`self.InventoryIDs`) ID)))
  (return (`|GetArrayItem` (`.Array_3_54825DA340DDAE3ADDAE89ABB7425895` (break `/Game/Blueprints/InventoryEquipment/Struct/S_ItemArray` (`BlueprintMapLibrary.Map_Find` (select `/Game/Blueprints/InventoryEquipment/Enum/E_ItemLocation` (`.ItemLocation_8_4E329D35476CDDB8E131009E226BCE64` (break `/Game/Blueprints/InventoryEquipment/Struct/S_ItemLocation` _output_get)) :`NewEnumerator0` (`self.InventoryArray`) :`NewEnumerator1` (`self.EquipmentArray`)) _itemtype))) _index)))

(fn `GetItemLocation`
  (params (ID :type Integer))
  (returns (Value :type "/Game/Blueprints/InventoryEquipment/Struct/S_ItemLocation Structure"))
  (return (`BlueprintMapLibrary.Map_Find` (`self.InventoryIDs`) ID)))

(fn `IsThereEmptySlotInEquipment`
  (params (ItemType :type "/Game/Blueprints/InventoryEquipment/Enum/E_ItemType Enum" :default "NewEnumerator0"))
  (returns (IsThere :type Boolean))
  (return (< (`KismetArrayLibrary.Array_Length` (`.Array_3_54825DA340DDAE3ADDAE89ABB7425895` (break `/Game/Blueprints/InventoryEquipment/Struct/S_ItemArray` (`BlueprintMapLibrary.Map_Find` (`self.EquipmentArray`) ItemType)))) (`BlueprintMapLibrary.Map_Find` (`self.EquipmentSlotsSizes`) ItemType))))

(fn `RemoveItemStats`
  (params (Item :type "/Game/Blueprints/InventoryEquipment/Struct/S_Item Structure"))
  (locals (Stat :type "/Game/Blueprints/InventoryEquipment/Struct/S_ItemStats Structure") (AmountsRef :type "Map of /Game/Blueprints/InventoryEquipment/Enum/E_StatAdditionType Enum to Float (double-precision)") (RemovedAmount :type "Float (double-precision)" :default 0.0))
  (bind ((`StatCategory_8_E8BBAE9D48BEC6D0801E889EF8F0BA87` _statcategory) (`StatAdditionType_2_29FFFC8F41736F431C31B68AAD5BE0B5` _statadditiontype)) (break `/Game/Blueprints/InventoryEquipment/Struct/S_ItemStats` (`local.Stat`)))
  (for _array_element (`.Stats_46_BD9FFE044F6D0BF1D424B09076C86854` (break `/Game/Blueprints/InventoryEquipment/Struct/S_Item` Item))
    (bind _output_get (set `local.Stat` _array_element))
    (bind (_statcategory_2 _statadditiontype_2 _statamount) (break `/Game/Blueprints/InventoryEquipment/Struct/S_ItemStats` _output_get))
    (bind _output_get_2 (set `local.AmountsRef` (`.Amounts_26_0915A13F4F6A65445893A8A768B38F02` (break `/Game/Blueprints/InventoryEquipment/Struct/S_StatAmounts` (`BlueprintMapLibrary.Map_Find` (`self.Stats`) _statcategory_2)))))
    (bind _output_get_3 (set `local.RemovedAmount` (- (`BlueprintMapLibrary.Map_Find` _output_get_2 _statadditiontype_2) _statamount)))
    (`BlueprintMapLibrary.Map_Add` (`local.AmountsRef`) _statadditiontype _output_get_3)
    (`BlueprintMapLibrary.Map_Add` (`self.Stats`) _statcategory (make `/Game/Blueprints/InventoryEquipment/Struct/S_StatAmounts` (`local.AmountsRef`))))
  (`self.StatsChanged` (`self.Stats`)))

(fn `SendItemToEquipment`
  (params (Item :type "/Game/Blueprints/InventoryEquipment/Struct/S_Item Structure"))
  (returns (Sended :type Boolean))
  (locals (ItemArrayRef :type "Array of /Game/Blueprints/InventoryEquipment/Struct/S_Item Structure") (ItemLocationRef :type "/Game/Blueprints/InventoryEquipment/Struct/S_ItemLocation Structure"))
  (bind (_itemlocation _itemtype _index) (break `/Game/Blueprints/InventoryEquipment/Struct/S_ItemLocation` (`BlueprintMapLibrary.Map_Find` (`self.InventoryIDs`) (`.ID_34_480AFE364D7F3357C84857B4B302F81E` (break `/Game/Blueprints/InventoryEquipment/Struct/S_Item` (`local.Item`))))))
  (bind _added (`self.AddItemToEquipment` Item))
  (if _added
    (bind _output_get (set `local.ItemArrayRef` (`.Array_3_54825DA340DDAE3ADDAE89ABB7425895` (break `/Game/Blueprints/InventoryEquipment/Struct/S_ItemArray` (`BlueprintMapLibrary.Map_Find` (`self.InventoryArray`) _itemtype)))))
    (`KismetArrayLibrary.Array_Remove` _output_get _index)
    (`BlueprintMapLibrary.Map_Add` (`self.InventoryArray`) (`.ItemType_35_B85020CC4326255BF9CA7986369ED08C` (break `/Game/Blueprints/InventoryEquipment/Struct/S_Item` (`local.Item`))) (make `/Game/Blueprints/InventoryEquipment/Struct/S_ItemArray` (`local.ItemArrayRef`)))
    (`self.ItemRemovedFromInventory` (`local.Item`))
    (return true)
    (else
      (return false))))

(fn `SendItemToInventory`
  (params (Item :type "/Game/Blueprints/InventoryEquipment/Struct/S_Item Structure"))
  (returns (Sended :type Boolean))
  (locals (ItemArrayRef :type "Array of /Game/Blueprints/InventoryEquipment/Struct/S_Item Structure") (ItemRef :type "/Game/Blueprints/InventoryEquipment/Struct/S_Item Structure"))
  (bind _output_get (set `local.ItemRef` Item))
  (bind _added (`self.AddItemToInventory` _output_get))
  (if _added
    (`self.RemoveItemStats` (`local.ItemRef`))
    (bind _output_get_2 (set `local.ItemArrayRef` (`.Array_3_54825DA340DDAE3ADDAE89ABB7425895` (break `/Game/Blueprints/InventoryEquipment/Struct/S_ItemArray` (`BlueprintMapLibrary.Map_Find` (`self.EquipmentArray`) (`.ItemType_35_B85020CC4326255BF9CA7986369ED08C` (break `/Game/Blueprints/InventoryEquipment/Struct/S_Item` (`local.ItemRef`))))))))
    (`KismetArrayLibrary.Array_Remove` _output_get_2 (`KismetArrayLibrary.Array_Find` _output_get_2 (`local.ItemRef`)))
    (`BlueprintMapLibrary.Map_Add` (`self.EquipmentArray`) (`.ItemType_35_B85020CC4326255BF9CA7986369ED08C` (break `/Game/Blueprints/InventoryEquipment/Struct/S_Item` (`local.ItemRef`))) (make `/Game/Blueprints/InventoryEquipment/Struct/S_ItemArray` (`local.ItemArrayRef`)))
    (`self.ItemRemovedFromEquipment` (`local.ItemRef`))
    (return true)
    (else
      (return false))))