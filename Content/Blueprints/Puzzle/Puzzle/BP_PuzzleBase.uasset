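; Base puzzle actor that removes itself when all of its completion conditions are already met.
; On BeginPlay it counts which ConditionsToComplete class tags appear in the GameInstance's CompletedConditionsTags, destroying the actor if every one is found.
; Interact runs the parent behavior, then passes each listed condition to AddCondition.
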(event `self.ReceiveBeginPlay`
  (bind _asbp_game_instance (cast `/Game/Blueprints/GameMode/BP_GameInstance` (`GameplayStatics.GetGameInstance`)))
  (for _array_element (`self.ConditionsToComplete`)
    (if (!= (`KismetArrayLibrary.Array_Find` (`/Game/Blueprints/GameMode/BP_GameInstance.CompletedConditionsTags` _asbp_game_instance) (`.ConditionTag` (defaults `Object` _array_element))) -1)
      (`/Engine/EditorBlueprintResources/StandardMacros.IncrementInt` (`self.CompletedConditionsCount`))))
  (if (== (`KismetArrayLibrary.Array_Length` (`self.ConditionsToComplete`)) (`self.CompletedConditionsCount`))
    (`self.K2_DestroyActor`)))

(event `/Game/Blueprints/Puzzle/Interface/BPI_Interact.Interact`
  (`parent.Interact`)
  (for _array_element (`self.ConditionsToComplete`)
    (`/Game/Blueprints/GeneralFunctions.AddCondition` _array_element)))

(fn `UserConstructionScript`)