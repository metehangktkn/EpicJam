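; BP_CheckKeyInInventory is a puzzle condition that completes when the player obtains a key.
; On BeginPlay it binds to the game instance's item-added-to-inventory event.
; When an added item is named "Key", it marks a floor as open and calls condition complete on itself.
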(event `self.ReceiveBeginPlay`
  (bind _asbp_game_instance (cast `/Game/Blueprints/GameMode/BP_GameInstance` (`GameplayStatics.GetGameInstance`)))
  (add `/Game/Blueprints/GameMode/BP_GameInstance.ItemAddedToInventory` _asbp_game_instance (`|CreateDelegate` :!event `CheckKey`)))

(event `CheckKey`
  (params (Item :type "/Game/Blueprints/InventoryEquipment/Struct/S_Item Structure"))
  (if (`KismetTextLibrary.EqualEqual_TextText` (`.Name_2_7F065C8A4B8C5E8DA4F3C1A4C1BBE804` (break `/Game/Blueprints/InventoryEquipment/Struct/S_Item` Item)) "Key")
    (`/Game/Blueprints/GeneralFunctions.SetFloorIsOpen` 1 true)
    (`self.ConditionComplete` self)))

(fn `UserConstructionScript`
  (`parent.UserConstructionScript`))